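; BP_ShootingHud is the shooting game's HUD Blueprint that passes local player state changes to the on-screen HUD widget.
; Update events for HP, ammo, magazine and user name each cast HudWidget to ShootingHudWidget and call its matching update function.
; The user name event calls UpdateUserName without passing the received name.
; HP, ammo and name events also print debug strings, while the magazine event does not.
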(event `self.OnUpdateMyHp`
  (params (CurHp :type "Float (single-precision)") (MaxHp :type "Float (single-precision)"))
  (`KismetSystemLibrary.PrintString` (`KismetStringLibrary.Concat_StrStr` "Update My CurHp : " (`KismetStringLibrary.Conv_DoubleToString` CurHp) ", MaxHp : " (`KismetStringLibrary.Conv_DoubleToString` MaxHp)))
  (bind _asshooting_hud_widget (cast `/Game/ShootingGame/Widget/ShootingHudWidget` (`self.HudWidget`)))
  (`/Game/ShootingGame/Widget/ShootingHudWidget.SetHp` _asshooting_hud_widget CurHp MaxHp))

(event `self.OnUpdateMyAmmo`
  (params (Ammo :type Integer))
  (`KismetSystemLibrary.PrintString` (`KismetStringLibrary.Concat_StrStr` "Update My Ammo - " (`KismetStringLibrary.Conv_IntToString` Ammo)))
  (bind _asshooting_hud_widget (cast `/Game/ShootingGame/Widget/ShootingHudWidget` (`self.HudWidget`)))
  (`/Game/ShootingGame/Widget/ShootingHudWidget.SetAmmo` _asshooting_hud_widget Ammo))

(event `self.OnUpdateMyMag`
  (params (Mag :type Integer))
  (bind _asshooting_hud_widget (cast `/Game/ShootingGame/Widget/ShootingHudWidget` (`self.HudWidget`)))
  (`/Game/ShootingGame/Widget/ShootingHudWidget.SetMag` _asshooting_hud_widget Mag))

(event `self.OnUpdateUserName`
  (params (UserName :type String))
  (`KismetSystemLibrary.PrintString` (`KismetStringLibrary.Concat_StrStr` "Update User Name - " UserName) true true (struct :`G` 0.66 :`B` 1.0 :`A` 1.0) 60.0)
  (bind _asshooting_hud_widget (cast `/Game/ShootingGame/Widget/ShootingHudWidget` (`self.HudWidget`)))
  (`/Game/ShootingGame/Widget/ShootingHudWidget.UpdateUserName` _asshooting_hud_widget))

(fn `UserConstructionScript`)